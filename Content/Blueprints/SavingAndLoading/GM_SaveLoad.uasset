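; Game mode that saves and restores per-level world state and player stats through SaveGame objects.
; On BeginPlay it loads the level save, in a slot named after the current level, and replays collected coins and opened doors on valid references.
; It also loads health, stamina and mana onto the third-person character from a shared player slot.
; Missing saves get fresh objects; separate events write each to disk.
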(event `self.ReceiveBeginPlay`
  (`KismetSystemLibrary.PrintText` "Loading the SavLoad Game mode" true true (struct :`R` 1.0 :`G` 0.386913 :`A` 1.0))
  (`self.LoadLevelStateFromFile`)
  (`self.LoadPlayerStats`))

(event `SaveLevelStateToFile`
  (bind _returnvalue (`GameplayStatics.GetCurrentLevelName` true))
  (bind _returnvalue_2 (`GameplayStatics.SaveGameToSlot` (`self.SG_LevelState`) _returnvalue))
  (if _returnvalue_2
    (`KismetSystemLibrary.PrintText` "Save Successful" true true (struct :`R` 0.021612 :`G` 1.0 :`A` 1.0) 5.0)
    (else
      (`KismetSystemLibrary.PrintText` "Failure to Save" true true (struct :`R` 1.0 :`B` 0.023286 :`A` 1.0) 5.0))))

(event `LoadLevelStateFromFile`
  (bind _returnvalue (`GameplayStatics.GetCurrentLevelName` true))
  (bind _returnvalue_2 (`GameplayStatics.DoesSaveGameExist` _returnvalue))
  (if _returnvalue_2
    (bind _returnvalue_3 (`GameplayStatics.LoadGameFromSlot` _returnvalue))
    (bind _assg_level_state (cast `/Game/Blueprints/SavingAndLoading/SG_LevelState` _returnvalue_3))
    (set `self.SG_LevelState` _assg_level_state)
    (`|ExecutionSequence`
      (:`then_0`
        (for _array_element (`/Game/Blueprints/SavingAndLoading/SG_LevelState.CollectedCoins` (`self.SG_LevelState`))
          (`/Engine/EditorBlueprintResources/StandardMacros.IsValid` _array_element ; Makes sure coins in other levels don't cause problems
            (:`Is Valid`
              (`/Game/Blueprints/BP_Coin.CollectSelf` _array_element)))))
      (:`then_1`
        (for _array_element_2 (`/Game/Blueprints/SavingAndLoading/SG_LevelState.OpenedDoors` (`self.SG_LevelState`))
          (`/Engine/EditorBlueprintResources/StandardMacros.IsValid` _array_element_2 ; Makes sure coins in other levels don't cause problems
            (:`Is Valid`
              (`/Game/Blueprints/BP_CameraDoor.OpenDoorNoCam` _array_element_2))))))
    (else
      (bind _returnvalue_4 (`GameplayStatics.CreateSaveGameObject` "/Game/Blueprints/SavingAndLoading/SG_LevelState.SG_LevelState_C"))
      (set `self.SG_LevelState` _returnvalue_4))))

(event `LoadPlayerStats`
  (bind _sg_playerstats (`self.SG_PlayerStats`))
  (bind _returnvalue (`GameplayStatics.DoesSaveGameExist` "PlayerSave"))
  (if _returnvalue
    (bind _returnvalue_2 (`GameplayStatics.LoadGameFromSlot` "PlayerSave"))
    (bind _assg_player_stats (cast `/Game/Blueprints/SavingAndLoading/SG_PlayerStats` _returnvalue_2))
    (set `self.SG_PlayerStats` _assg_player_stats)
    (bind _asbp_third_person_character (cast `/Game/ThirdPerson/Blueprints/BP_ThirdPersonCharacter` (`GameplayStatics.GetPlayerCharacter` 0)))
    (set `/Game/ThirdPerson/Blueprints/BP_ThirdPersonCharacter.Stamina` (`/Game/Blueprints/SavingAndLoading/SG_PlayerStats.Stamina` _sg_playerstats) _asbp_third_person_character)
    (set `/Game/ThirdPerson/Blueprints/BP_ThirdPersonCharacter.Health` (`/Game/Blueprints/SavingAndLoading/SG_PlayerStats.HealthP` _sg_playerstats) _asbp_third_person_character)
    (set `/Game/ThirdPerson/Blueprints/BP_ThirdPersonCharacter.Mana` (`/Game/Blueprints/SavingAndLoading/SG_PlayerStats.ManaP` _sg_playerstats) _asbp_third_person_character)
    (`KismetSystemLibrary.PrintText` "Player Stats have been loaded" true true (struct :`R` 1.0 :`G` 0.386913 :`A` 1.0))
    (else
      (bind _returnvalue_3 (`GameplayStatics.CreateSaveGameObject` "/Game/Blueprints/SavingAndLoading/SG_PlayerStats.SG_PlayerStats_C"))
      (set `self.SG_PlayerStats` _returnvalue_3))))

(event `SavePlayerStats`
  (bind _returnvalue (`GameplayStatics.SaveGameToSlot` (`self.SG_PlayerStats`) "PlayerSave"))
  (if _returnvalue
    (`KismetSystemLibrary.PrintText` "Player Stats written to file" true true (struct :`R` 0.021876 :`G` 1.0 :`A` 1.0))
    (else
      (`KismetSystemLibrary.PrintText` "Player Stats write fail" true true (struct :`R` 1.0 :`A` 1.0)))))

(fn `UserConstructionScript`)