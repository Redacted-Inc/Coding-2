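; BP_EnemySpawnManager populates the level with AI enemies when play begins.
; It finds every BP_EnemySpawnPoint, prints the count, and gives each a weighted random chance to spawn a BP_AiMoveTo at its transform.
; Each spawned AI gets a random name from a hardcoded list and randomly picked dynamic material instances on its first two mesh slots.
; A final random branch leads to no action.
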(event `self.ReceiveBeginPlay`
  (bind _outactors (`GameplayStatics.GetAllActorsOfClass` "/Game/Blueprints/BP_EnemySpawnPoint.BP_EnemySpawnPoint_C"))
  (`KismetSystemLibrary.PrintText` (`|FormatText` "There are {count} spawn points" (`KismetArrayLibrary.Array_Length` _outactors)))
  (for _array_element _outactors
    (if (`KismetMathLibrary.RandomBoolWithWeight` 0.75)
      (bind _returnvalue (`|SpawnActorFromClass` "/Game/AI_Blueprints/BP_AiMoveTo.BP_AiMoveTo_C" (`self.GetTransform` _array_element) "Undefined" "MultiplyWithRoot" _array_element null))
      (`TextRenderComponent.K2_SetText` (`/Game/AI_Blueprints/BP_AiMoveTo.AI_Name_Text` _returnvalue) (`|GetArrayItem` (`|MakeArray` "THE DESTROYER" "bob!" "Gargamel" "Elvion" "Bleezlebob" "Howard Antiqurius Von Jaegermiester III" :!type "Text") (`KismetMathLibrary.RandomInteger` 6)))
      (bind _returnvalue_2 (`KismetMaterialLibrary.CreateDynamicMaterialInstance` "/Game/Materials/MI_EmissivePink.MI_EmissivePink"))
      (bind _returnvalue_3 (`KismetMaterialLibrary.CreateDynamicMaterialInstance` "/Game/Materials/MI_FlatYellow.MI_FlatYellow"))
      (bind _returnvalue_4 (`KismetMaterialLibrary.CreateDynamicMaterialInstance` "/Game/Footsteps/MI_Grass.MI_Grass"))
      (bind _returnvalue_5 (`KismetMaterialLibrary.CreateDynamicMaterialInstance` "/Game/Materials/MI_FlatBlack.MI_FlatBlack"))
      (bind _mesh (`Character.Mesh` _returnvalue))
      (bind _array (`|MakeArray` _returnvalue_2 _returnvalue_3 _returnvalue_4 _returnvalue_5))
      (`PrimitiveComponent.SetMaterial` _mesh 0 (`|GetArrayItem` _array (`KismetMathLibrary.RandomInteger` 4)))
      (`PrimitiveComponent.SetMaterial` _mesh 1 (`|GetArrayItem` _array (`KismetMathLibrary.RandomInteger` 4)))
      (if (`KismetMathLibrary.RandomBool`)
        _))))

(fn `UserConstructionScript`)