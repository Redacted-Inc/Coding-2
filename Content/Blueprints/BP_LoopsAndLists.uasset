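; BP_LoopsAndLists is a Blueprint demo of loop types and color arrays that prints its results to the screen.
; BeginPlay starts a self-rewiring Delay and DoN cycle, which prints its run count and fires a colored ForLoop on each timed pass until the limit.
; WhileLoop (self-resetting countdown) and ForEachLoop (color array) examples are also defined, but their calls are disconnected and never run.
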(event `self.ReceiveBeginPlay`
  (`KismetSystemLibrary.PrintString` "Loops and Lists Exist")
  (`self.DelayLoop`))

(event `DelayLoop`
  (`KismetSystemLibrary.PrintString` "Starting Delay Looop")
  (`KismetSystemLibrary.Delay` 1.0 :!label _label)
  (bind _counter (`/Engine/EditorBlueprintResources/StandardMacros.Do N` 20)
    (:`Exit`
      (`KismetSystemLibrary.PrintText` (`|FormatText` "This has run {count} times" _counter) true true (struct :`R` 1.0 :`G` 0.885933 :`A` 1.0))
      (`self.StartForLoop`)
      (goto _label))))

(event `StartForLoop`
  (bind _array (`|MakeArray` (struct :`R` 1.0 :`G` 0.366049 :`A` 1.0) (struct :`R` 0.226364 :`B` 0.273958 :`A` 1.0) (struct :`R` 0.011904 :`G` 0.265625 :`A` 1.0) (struct :`R` 0.045135 :`B` 1.0 :`A` 1.0) (struct :`R` 0.578125 :`G` 0.009222 :`B` 3.7e-05 :`A` 1.0) (struct :`R` 1.0 :`G` 0.986161 :`B` 0.837423 :`A` 1.0) :!type "LinearColor Structure"))
  (for _index (range (`KismetArrayLibrary.Array_Length` _array))
    (`KismetSystemLibrary.PrintText` (`|FormatText` "This is Index #{index}" _index) true true (`|GetArrayItem` _array _index))))

(event `StartWhileLoop`
  (while (> (`self.WhileLoopCounter`) 0)
    (`KismetSystemLibrary.PrintText` (`|FormatText` "There are {count} more runs of this loop" (`self.WhileLoopCounter`)) true true (struct :`R` 1.0 :`B` 0.880133 :`A` 1.0))
    (`/Engine/EditorBlueprintResources/StandardMacros.DecrementInt` (`self.WhileLoopCounter`)))
  (set `self.WhileLoopCounter` 10))

(event `StartForEachLoop`
  (for (_array_element _array_index) (`|MakeArray` (struct :`R` 1.0 :`G` 0.366049 :`A` 1.0) (struct :`R` 0.226364 :`B` 0.273958 :`A` 1.0) (struct :`R` 0.011904 :`G` 0.265625 :`A` 1.0) (struct :`R` 0.045135 :`B` 1.0 :`A` 1.0) :!type "LinearColor Structure")
    (`KismetSystemLibrary.PrintText` (`|FormatText` "This is Index #{index}" _array_index) true true _array_element)))

(fn `UserConstructionScript`)